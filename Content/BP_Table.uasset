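; Interactable table where the player places a pizza box and then opens it, driven by a Step counter in OnInteract.
; The first interaction requires a visible image on the first-person HUD's food indicator, notifies that widget, sets the box mesh and advances Step.
; The next swaps to the following PizzaBox mesh and reveals the pizza attached to its "Contained" socket.
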(fn `OnInteract`
  (params (Interactor :type "MiniJamCharacter Object Reference"))
  (returns (ReturnValue :type Boolean))
  (bind _pizzza (`self.Pizzza`))
  (bind _left (`self.Left`))
  (bind _step (`self.step`))
  (bind _output (`|GetArrayItem` (`self.PizzaBox`) _step))
  (switch `int` _step
    (:`Default`
      _)
    (:`0`
      ;[1 0.15 0.15] Pizza Placing (0)
      (bind _asfirst_person_character (cast `/Game/FirstPersonCPP/Blueprints/FirstPersonCharacter` Interactor))
      (bind _asplayer_controller (cast `PlayerController` (`Pawn.GetController` _asfirst_person_character)))
      (bind _asfirst_person_hud (cast `/Game/FirstPersonHUD` (`PlayerController.GetHUD` _asplayer_controller)))
      (bind _foodindicatorref (`/Game/FirstPersonHUD.FoodIndicatorref` _asfirst_person_hud))
      (if (`Widget.IsVisible` (`/Game/WBP_FoodIndicator.Image_36` _foodindicatorref))
        (`/Game/WBP_FoodIndicator.OnPlaced` _foodindicatorref)
        (bind _returnvalue (`StaticMeshComponent.SetStaticMesh` _left _output))
        (set `self.step` (+ _step 1))))
    (:`1`
      ;[1 0.3625 0.15] Open Pizza Box (1)
      (`StaticMeshComponent.SetStaticMesh` _left _output)
      (`SceneComponent.K2_AttachToComponent` _pizzza _left "Contained" "KeepRelative" "KeepRelative" "KeepRelative" true)
      (`SceneComponent.SetVisibility` _pizzza true false)))
  (return _returnvalue))

(fn `UserConstructionScript`)