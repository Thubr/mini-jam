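; A door actor that swings open when the FirstPersonCharacter enters its Front trigger and closes when the character leaves.
; Overlap events play separate open and close timelines that drive the door's yaw, with DoOnce gates reset on timeline updates.
; IsFacingArrow uses dot-product angles between door, actor and their forward vectors to pick the swing direction, reused on closing, and prints debug values.
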(event `self.Front.OnComponentBeginOverlap`
  (params (OverlappedComponent :type "PrimitiveComponent Object Reference") (OtherActor :type "Actor Object Reference") (OtherComp :type "PrimitiveComponent Object Reference") (OtherBodyIndex :type Integer) (bFromSweep :type Boolean) (SweepResult :type "HitResult Structure (by ref)"))
  (bind _isfacing (`self.Is Facing Arrow` OtherActor))
  (`KismetSystemLibrary.PrintString` (`KismetStringLibrary.Conv_BoolToString` _isfacing))
  (cast `/Game/FirstPersonCPP/Blueprints/FirstPersonCharacter` OtherActor)
  (`/Engine/EditorBlueprintResources/StandardMacros.DoOnce` false :!label _label
    (:`Completed`
      (bind (_direction _opening) (`Timeline|OpenDoor` :!via `PlayFromStart`)
        (:`Update`
          (`SceneComponent.K2_SetRelativeRotation` (`self.Door`) (`KismetMathLibrary.MakeRotator` 0.0 0.0 (select `bool` _isfacing :`false` _opening :`true` (* -1 _opening))) false false)
          (goto _label :!via `Reset`))))))

(event `self.Front.OnComponentEndOverlap`
  (params (OverlappedComponent :type "PrimitiveComponent Object Reference") (OtherActor :type "Actor Object Reference") (OtherComp :type "PrimitiveComponent Object Reference") (OtherBodyIndex :type Integer))
  (cast `/Game/FirstPersonCPP/Blueprints/FirstPersonCharacter` OtherActor)
  (`/Engine/EditorBlueprintResources/StandardMacros.DoOnce` false :!label _label_2
    (:`Completed`
      (bind (_direction _closing) (`Timeline|CloseDoor` :!via `PlayFromStart`)
        (:`Update`
          (`SceneComponent.K2_SetRelativeRotation` (`self.Door`) (`KismetMathLibrary.MakeRotator` 0.0 0.0 (select `bool` (stale `self.Front.OnComponentBeginOverlap` _isfacing) :`false` _closing :`true` (* -1 _closing))) false false)
          (goto _label_2 :!via `Reset`))))))

(fn `Is Facing Arrow`
  (params (Actor :type "Actor Object Reference"))
  (returns (IsFacing :type Boolean))
  (bind _returnvalue (`self.K2_GetActorLocation` Actor))
  (bind _door (`self.Door`))
  (bind _returnvalue_2 (`SceneComponent.K2_GetComponentLocation` _door))
  (bind _returnvalue_3 (`KismetMathLibrary.DegAcos` (`KismetMathLibrary.Dot_VectorVector` (`KismetMathLibrary.Normal` (- _returnvalue _returnvalue_2)) (`SceneComponent.GetForwardVector` _door))))
  (bind _returnvalue_4 (`KismetMathLibrary.DegAcos` (`KismetMathLibrary.Dot_VectorVector` (`KismetMathLibrary.Normal` (- _returnvalue_2 _returnvalue)) (`self.GetActorForwardVector` Actor))))
  (`KismetSystemLibrary.PrintString` (`KismetStringLibrary.Conv_DoubleToString` _returnvalue_3))
  (`KismetSystemLibrary.PrintString` (`KismetStringLibrary.Conv_DoubleToString` _returnvalue_4))
  (return (and (and (<= _returnvalue_3 105.0) (>= _returnvalue_3 0.0)) (and (<= _returnvalue_4 105.0) (>= _returnvalue_4 0.0)))))

(fn `UserConstructionScript`)