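; BP_Pizza is an interactable pizza pickup that the player collects.
; OnInteract resolves the interactor's player controller, then on the first step notifies the FirstPersonHUD's food indicator via OnCollect and hides the actor.
; A PizzaStep counter then advances so later interactions skip collection and simply return true.
; The actor is hidden rather than destroyed.
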(fn `OnInteract`
  (params (Interactor :type "MiniJamCharacter Object Reference"))
  (returns (ReturnValue :type Boolean))
  (bind _asplayer_controller (cast `PlayerController` (`Pawn.GetController` Interactor)))
  (switch `int` (`self.pizzaStep`)
    (:`Default`
      _)
    (:`0`
      (bind _asfirst_person_hud (cast `/Game/FirstPersonHUD` (`PlayerController.GetHUD` _asplayer_controller)))
      (`/Game/WBP_FoodIndicator.OnCollect` (`/Game/FirstPersonHUD.FoodIndicatorref` _asfirst_person_hud))
      (`self.SetActorHiddenInGame` true)
      (set `self.pizzaStep` 1)))
  (return true))

(fn `UserConstructionScript`)