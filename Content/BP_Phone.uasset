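; BP_Phone is an interactable phone that opens a phone UI when the player presses F nearby.
; A box overlap with the FirstPersonCharacter sets an in-range flag and toggles a text render prompt.
; The phone HUD widget is created on BeginPlay, then on F it is added to the viewport with UI-only input, a visible cursor and the game paused.
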(event `self.ReceiveBeginPlay`
  (bind _output_get (set `self.PlayerController` (`GameplayStatics.GetPlayerController` 0)))
  (`self.EnableInput` _output_get)
  (bind _returnvalue (`|CreateWidget` "/Game/WBP_PhoneHUD.WBP_PhoneHUD_C"))
  (set `self.PhoneWidgetRef` _returnvalue))

(event `Key|F`
  (params (Key :type "Key Structure"))
  (bind _phonewidgetref (`self.PhoneWidgetRef`))
  (bind _playercontroller (`self.PlayerController`))
  ;[1 1 1] Interaction
  (:`Pressed`
    (if (`self.InRange`)
      (`WidgetBlueprintLibrary.SetInputMode_UIOnlyEx` _playercontroller _phonewidgetref)
      (set `PlayerController.bShowMouseCursor` true _playercontroller)
      (`UserWidget.AddToViewport` _phonewidgetref 0)
      (`GameplayStatics.SetGamePaused` true))))

(event `self.Box.OnComponentBeginOverlap`
  (params (OverlappedComponent :type "PrimitiveComponent Object Reference") (OtherActor :type "Actor Object Reference") (OtherComp :type "PrimitiveComponent Object Reference") (OtherBodyIndex :type Integer) (bFromSweep :type Boolean) (SweepResult :type "HitResult Structure (by ref)"))
  ;[1 0.205 0.4083] Trigger Overlap
  (bind _asfirst_person_character (cast `/Game/FirstPersonCPP/Blueprints/FirstPersonCharacter` OtherActor))
  (set `self.InRange` true)
  (set `self.As First Person Character` _asfirst_person_character)
  (`SceneComponent.SetVisibility` (`self.TextRender`) true false))

(event `self.Box.OnComponentEndOverlap`
  (params (OverlappedComponent :type "PrimitiveComponent Object Reference") (OtherActor :type "Actor Object Reference") (OtherComp :type "PrimitiveComponent Object Reference") (OtherBodyIndex :type Integer))
  ;[1 0.205 0.4083] Trigger Overlap
  (cast `/Game/FirstPersonCPP/Blueprints/FirstPersonCharacter` OtherActor)
  (set `self.InRange` false)
  (`SceneComponent.SetVisibility` (`self.TextRender`) false false))

(fn `UserConstructionScript`)